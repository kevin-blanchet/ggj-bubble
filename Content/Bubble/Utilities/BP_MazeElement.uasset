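; BP_MazeElement is one cell of a 3D maze, with six walls and an optional exit bubble.
; Its UpdateWalls event destroys each wall component whose flag is false, then teleports the actor to its grid coordinate scaled by the element size.
; It also destroys the exit bubble component unless the cell is marked as the exit.
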(event `self.UpdateWalls`
  (`|ExecutionSequence`
    (:`then_0`
      (if (not (`self.bLeftWall`))
        (`ActorComponent.K2_DestroyComponent` (`self.LeftWall`))))
    (:`then_1`
      (if (not (`self.bRightWall`))
        (`ActorComponent.K2_DestroyComponent` (`self.RightWall`))))
    (:`then_2`
      (if (not (`self.bTopWall`))
        (`ActorComponent.K2_DestroyComponent` (`self.TopWall`))))
    (:`then_3`
      (if (not (`self.bBottomWall`))
        (`ActorComponent.K2_DestroyComponent` (`self.BottomWall`))))
    (:`then_4`
      (if (not (`self.bFrontWall`))
        (`ActorComponent.K2_DestroyComponent` (`self.FrontWall`))))
    (:`then_5`
      (if (not (`self.bBackWall`))
        (`ActorComponent.K2_DestroyComponent` (`self.BackWall`))))
    (:`then_6`
      (`self.K2_SetActorTransform` (`KismetMathLibrary.MakeTransform` (* (`self.Coord`) (`self.elementSize`))) false true))
    (:`then_7`
      (if (not (`self.bIsExit`))
        (`ActorComponent.K2_DestroyComponent` (`self.BP_ExitBubble`))))))

(fn `UserConstructionScript`)